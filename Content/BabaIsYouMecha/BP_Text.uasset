(event EventBeginPlay
  (|SetMaterialByCondition
    (:ExecOut
      (CallFunction|SetTag))))

(event OnComponentBeginOverlap(Box1)
  (params (OverlappedComponent :type Primitive%20Component%20Object%20Reference) (OtherActor :type Actor%20Object%20Reference) (OtherComp :type Primitive%20Component%20Object%20Reference) (OtherBodyIndex :type Integer) (bFromSweep :type Boolean) (SweepResult :type Hit%20Result%20Structure%20%28by%20ref%29)))

(event OnComponentBeginOverlap(Box2)
  (params (OverlappedComponent :type Primitive%20Component%20Object%20Reference) (OtherActor :type Actor%20Object%20Reference) (OtherComp :type Primitive%20Component%20Object%20Reference) (OtherBodyIndex :type Integer) (bFromSweep :type Boolean) (SweepResult :type Hit%20Result%20Structure%20%28by%20ref%29)))

(event OnComponentBeginOverlap(Box3)
  (params (OverlappedComponent :type Primitive%20Component%20Object%20Reference) (OtherActor :type Actor%20Object%20Reference) (OtherComp :type Primitive%20Component%20Object%20Reference) (OtherBodyIndex :type Integer) (bFromSweep :type Boolean) (SweepResult :type Hit%20Result%20Structure%20%28by%20ref%29)))

(event OnComponentBeginOverlap(Box4)
  (params (OverlappedComponent :type Primitive%20Component%20Object%20Reference) (OtherActor :type Actor%20Object%20Reference) (OtherComp :type Primitive%20Component%20Object%20Reference) (OtherBodyIndex :type Integer) (bFromSweep :type Boolean) (SweepResult :type Hit%20Result%20Structure%20%28by%20ref%29)))

(event Custom|SetTag
  (Variables|Default|SetTags (Utilities|Array|MakeArray (Utilities|Select :Index (Variables|Parameter|GetE_Condition) :NewEnumerator0 "Object" :NewEnumerator1 "Condition" :NewEnumerator2 "Fonction" :NewEnumerator3 "Object" :NewEnumerator4 "Fonction"))))

(event EventTick
  (params (DeltaSeconds :type Float%20%28single-precision%29))
  (for _array_element (Variables|Actor|GetTags)
    _)
  (if (== _array_element "Object")
    _))

(fn ConstructionScript)

(fn SudTrace
  (bind _cube (Variables|Default|GetCube))
  (bind _returnvalue (Transformation|GetWorldLocation _cube))
  (bind (_outhits _returnvalue_2) (Class|KismetSystemLibrary|LineTraceMultiforObjects _returnvalue (+ _returnvalue (* (Math|Vector|GetForwardVector (Variables|Default|GetArrowSud)) 4e+02)) (Utilities|Array|MakeArray "ObjectTypeQuery2") true (Utilities|Array|MakeArray self) "ForOneFrame" true))
  (if _returnvalue_2
    (for _array_element _outhits
      (Variables|Default|SetHitActor (Utilities|Array|MakeArray (.HitActor (Collision|BreakHitResult _array_element))))
      (return))))

(fn OuestTrace
  (bind _cube (Variables|Default|GetCube))
  (bind _returnvalue (Transformation|GetWorldLocation _cube))
  (bind _outhits (Class|KismetSystemLibrary|LineTraceMultiforObjects _returnvalue (+ _returnvalue (* (Math|Vector|GetForwardVector (Variables|Default|GetArrowOuest)) 4e+02)) (Utilities|Array|MakeArray "ObjectTypeQuery2") true (Utilities|Array|MakeArray self) "ForOneFrame" true))
  (for _array_element _outhits
    _))