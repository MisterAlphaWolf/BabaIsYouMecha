(event EventBeginPlay
  (Variables|Default|SetLinear%20Color (Utilities|Struct|MakeLinearColor (Math|Random|RandomFloat) (Math|Random|RandomFloat) (Math|Random|RandomFloat) 1.0)))

(event EventTick
  (params (DeltaSeconds :type Float%20%28single-precision%29))
  (bind _linear_color (Variables|Default|GetLinear%20Color))
  (Utilities|FlowControl|Sequence
    (:then_0
      (bind _hitactor (|LineTraceSud))
      (|DebugSud _hitactor _linear_color)
      (Variables|TextHit|SetHitActorSud _hitactor))
    (:then_1
      (bind _hitactor_2 (|LineTraceNord))
      (|DebugNord _hitactor_2 _linear_color)
      (Variables|TextHit|SetHitActorNord _hitactor_2))
    (:then_2
      (bind _hitactor_3 (|LineTraceEst))
      (|DebugEst _hitactor_3 _linear_color)
      (Variables|TextHit|SetHitActorEst _hitactor_3))
    (:then_3
      (bind _hitactor_4 (|LineTraceOuest))
      (|DebugOuest _hitactor_4 _linear_color)
      (Variables|TextHit|SetHitActorOuest _hitactor_4))))

(fn ConstructionScript)